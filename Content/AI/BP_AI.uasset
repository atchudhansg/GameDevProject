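; BP_AI is an AI character Blueprint with basic health, death and attack behavior.
; Incoming damage lowers Health, and at zero or below the mesh switches to physics simulation as a ragdoll-style death.
; An Attack event plays an attack montage on the mesh; nothing in this file triggers it or applies damage.
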(event EventAttack
  (Animation|Montage|PlayMontage (Variables|Character|GetMesh) "/Game/Characters/Mannequins/Animations/Attack_Montage.Attack_Montage"))

(event Game|Damage|EventAnyDamage
  (params (Damage :type Float%20%28single-precision%29) (DamageType :type Damage%20Type%20Object%20Reference) (InstigatedBy :type Controller%20Object%20Reference) (DamageCauser :type Actor%20Object%20Reference))
  (Variables|Default|Sethealth (- (Variables|Default|Gethealth) Damage))
  (if (<= (Variables|Default|Gethealth) 0.0)
    (Physics|SetSimulatePhysics (Variables|Character|GetMesh) true)))

(fn ConstructionScript)